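; AirPlane is a keyboard-steered plane Blueprint that flies forward constantly along its root's forward vector.
; The Helice macro spins the propeller each Tick and passes DeltaSeconds to Move, which offsets the root without sweep.
; A/D set YRot, applied as per-frame roll without delta-time scaling.
; W/S set XRot, but nothing reads it, so pitch stays unchanged.
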(event EventBeginPlay)

(event Collision|EventActorBeginOverlap
  (params (OtherActor :type Actor%20Object%20Reference)))

(event Input|KeyboardEvents|W
  (params (Key :type Key%20Structure))
  (:Pressed
    (Variables|Default|SetXRot 1.0))
  (:Released
    (Variables|Default|SetXRot 0.0)))

(event Input|KeyboardEvents|S
  (params (Key :type Key%20Structure))
  (:Pressed
    (Variables|Default|SetXRot -1.0))
  (:Released
    (Variables|Default|SetXRot 0.0)))

(event Input|KeyboardEvents|A
  (params (Key :type Key%20Structure))
  (:Pressed
    (Variables|Default|SetYRot -1.0))
  (:Released
    (Variables|Default|SetYRot 0.0)))

(event Input|KeyboardEvents|D
  (params (Key :type Key%20Structure))
  (:Pressed
    (Variables|Default|SetYRot 1.0))
  (:Released
    (Variables|Default|SetYRot 0.0)))

(fn ConstructionScript)

(event EventTick
  (params (DeltaSeconds :type Float%20%28single-precision%29))
  (Transformation|AddRelativeRotation (Variables|Default|GetPropeller) "42.000000, 0, 0" false false)
  (return DeltaSeconds))